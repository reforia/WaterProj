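; BP_WaterCore is a water body actor that builds a water surface and the post-process box beneath it in its construction script.
; WaterPlaneProportion sets the instanced-mesh plane's height within WaterVolume, and the post-process box is fitted from the volume's bottom to that plane.
; When Unbound, the plane becomes a centered grid of instances, and the box's horizontal extent derives from the instance count.
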(event EventBeginPlay)

(event Collision|EventActorBeginOverlap
  (params (OtherActor :type Actor%20Object%20Reference)))

(event EventTick
  (params (DeltaSeconds :type Float%20%28single-precision%29)))

(fn ConstructionScript
  ;[1 1 1] Initialization
  (CallFunction|SetWaterPlaneZ (Variables|Water|GetWaterPlaneProportion))
  (CallFunction|SetPostProcessZ (Variables|Default|GetInstancedStaticMesh))
  (CallFunction|ScaleWaterPlane (Variables|General|GetUnbound))
  (CallFunction|ScalePostProcess (Variables|General|GetUnbound)))

(fn SetWaterPlaneZ
  (params (HeightProportion :type Float%20%28single-precision%29))
  (Transformation|SetRelativeLocation (Variables|Default|GetInstancedStaticMesh) (Math|Vector|MakeVector 0.0 0.0 (* (.z (Components|Box|GetScaledBoxExtent (Variables|Default|GetWaterVolume))) (+ (* HeightProportion 2.0) -1.0) (/ 1.0 (.z (Transformation|GetActorScale3D))))) false false))

(fn ScaleWaterPlane
  (params (Unbound :type Boolean))
  (bind _i (LocalVariables|GetI))
  (bind _returnvalue (* _i -5e+01))
  (bind _returnvalue_2 (+ _returnvalue 5e+01))
  (if Unbound
    (for _index (range 0 (- (LocalVariables|GetI) 1))
      (for _index_2 (range 0 (- (LocalVariables|GetI) 1))
        (Components|InstancedStaticMesh|AddInstance (Variables|Default|GetInstancedStaticMesh) (Math|Transform|MakeTransform (Math|Vector|MakeVector (* (Math|Conversions|ToFloat(Integer) _index_2) 1e+02) (* (Math|Conversions|ToFloat(Integer) _index) 1e+02) 0.0) "0, 0, 0" "1,1,1"))))
    (Transformation|AddLocalOffset (Variables|Default|GetInstancedStaticMesh) (Math|Vector|MakeVector _returnvalue_2 _returnvalue_2 0.0) false false)
    (else
      (Components|InstancedStaticMesh|AddInstance (Variables|Default|GetInstancedStaticMesh) (Math|Transform|MakeTransform "0.0,0.0,0.0" "0, 0, 0" "1,1,1")))))

(fn ScalePostProcess
  (params (UnBound :type Boolean))
  (bind _instancedstaticmesh (Variables|Default|GetInstancedStaticMesh))
  (bind _postprocessvolume (Variables|Default|GetPostProcessVolume))
  (bind _returnvalue (Components|InstancedStaticMesh|GetInstanceCount _instancedstaticmesh))
  (bind _boxextent (Variables|/Script/Engine.BoxComponent|GetBoxExtent _postprocessvolume))
  (bind _returnvalue_2 (Math|Conversions|ToFloat(Integer) _returnvalue))
  (bind _returnvalue_3 (Math|Float|Sqrt _returnvalue_2))
  (bind _returnvalue_4 (* _returnvalue_3 0.5 1e+02))
  (Components|Box|SetBoxExtent _postprocessvolume (select UnBound (Math|Vector|MakeVector _returnvalue_4 _returnvalue_4 (.Z (Math|Vector|BreakVector _boxextent))) _boxextent) true))

(fn SetPostProcessZ
  (params (WaterPlaneRef :type Static%20Mesh%20Component%20Object%20Reference))
  (bind _relativelocation (Variables|/Script/Engine.SceneComponent|GetRelativeLocation WaterPlaneRef))
  (bind _watervolume (Variables|Default|GetWaterVolume))
  (bind _watervolume_2 (Variables|Default|GetWaterVolume))
  (bind _returnvalue (Components|Box|GetUnscaledBoxExtent _watervolume))
  (bind _returnvalue_2 (Components|Box|GetUnscaledBoxExtent _watervolume_2))
  (bind _returnvalue_3 (+ (.z _returnvalue) (.z _relativelocation)))
  (bind _returnvalue_4 (* _returnvalue_3 0.5))
  ;[1 1 1] Set Center of PP
  (Transformation|SetRelativeLocation (Variables|Default|GetPostProcessVolume) (Math|Vector|MakeVector 0.0 0.0 (- (.z _relativelocation) _returnvalue_4)) false false)
  ;[1 1 1] Set Extent
  (Components|Box|SetBoxExtent (Variables|Default|GetPostProcessVolume) (Math|Vector|MakeVector (.x _returnvalue_2) (.y _returnvalue_2) _returnvalue_4) true))